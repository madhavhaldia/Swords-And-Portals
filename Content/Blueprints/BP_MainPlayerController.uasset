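; BP_MainPlayerController is a player controller Blueprint that animates the pause menu as it opens and closes.
; It extends the parent's display and remove events, then casts PauseMenu to BP_PauseMenu to play its PauseMenuAnimation.
; Opening plays the animation forward; closing plays it in reverse and hides the widget after a short fixed delay.
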(event EventRemovePauseMenu
  (|CallParentFunction)
  (bind _asbp_pause_menu (Utilities|Casting|CastToBP_PauseMenu (Variables|Default|GetPauseMenu)))
  (UserInterface|Animation|PlayAnimation _asbp_pause_menu (Variables|/Game/HUD/BP_PauseMenu.BP_PauseMenu_C|GetPauseMenuAnimation _asbp_pause_menu) 0.0 1 "Reverse" 1.0 false)
  (Utilities|FlowControl|Delay 0.5)
  (Widget|SetVisibility (Variables|Default|GetPauseMenu) "Hidden"))

(event EventDisplayPauseMenu
  (|CallParentFunction)
  (bind _asbp_pause_menu (Utilities|Casting|CastToBP_PauseMenu (Variables|Default|GetPauseMenu)))
  (UserInterface|Animation|PlayAnimation _asbp_pause_menu (Variables|/Game/HUD/BP_PauseMenu.BP_PauseMenu_C|GetPauseMenuAnimation _asbp_pause_menu) 0.0 1 "Forward" 1.0 false))

(fn ConstructionScript)